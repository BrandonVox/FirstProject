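; BP_Cube is an actor that bobs vertically in a sine wave around the location it has at BeginPlay.
; Each Tick, UpdateSeconds accumulates elapsed time and feeds it to TanHeightAdder, which despite its name applies Sin, scaled by SpeedMultiplier and HeightMultiplier.
; The actor's location is set to the stored start position plus that Z offset, without sweep or teleport.
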(event EventTick
  (params (DeltaSeconds :type Float%20%28single-precision%29))
  (bind _updatedseconds (CallFunction|UpdateSeconds DeltaSeconds))
  (Transformation|SetActorLocation (+ (Variables|Default|GetBeginLocation) (Math|Vector|MakeVector 0.0 0.0 (CallFunction|TanHeightAdder _updatedseconds))) false false))

(event EventBeginPlay
  (Variables|Default|SetBeginLocation (Transformation|GetActorLocation)))

(fn ConstructionScript)

(fn TanHeightAdder
  (params (SampleValue :type Float%20%28double-precision%29))
  (return (* (Math|Trig|Sin(Radians) (* SampleValue (Variables|Movement|GetSpeedMultiplier))) (Variables|Movement|GetHeightMultiplier))))

(fn UpdateSeconds
  (params (DeltaSeconds :type Float%20%28double-precision%29))
  (bind _output_get (Variables|Default|SetSeconds (+ (Variables|Default|GetSeconds) DeltaSeconds)))
  (return _output_get))